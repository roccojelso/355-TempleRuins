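; Lever Blueprint that sends TogglebleObject on and off messages to the linked OtherActorsAreControlledByThisActor reference.
; Box overlap begin enables player input and calls TurnOnMessage; overlap end disables input and calls TurnOffMessage after an interface check.
; F press flips LeverPulled, which is never read here, and reruns the on path.
; F release runs the off path, which also disables input.
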(event `self.Box.OnComponentBeginOverlap`
  (params (OverlappedComponent :type "PrimitiveComponent Object Reference") (OtherActor :type "Actor Object Reference") (OtherComp :type "PrimitiveComponent Object Reference") (OtherBodyIndex :type Integer) (bFromSweep :type Boolean) (SweepResult :type "HitResult Structure (by ref)"))
  (bind _other_actors_are_controlled_by_this_actor (`self.Other Actors are controlled by this Actor`))
  (`/Engine/EditorBlueprintResources/StandardMacros.IsValid` _other_actors_are_controlled_by_this_actor :!label _label
    (:`Is Valid`
      (if true
        (`self.EnableInput` (`GameplayStatics.GetPlayerController` 0))
        (message `/Game/Blueprints/TogglebleObject.Turn On` _other_actors_are_controlled_by_this_actor null)))))

(event `Key|F`
  (params (Key :type "Key Structure"))
  (bind _other_actors_are_controlled_by_this_actor (`self.Other Actors are controlled by this Actor`))
  (:`Pressed`
    (set `self.Lever Pulled` (not (`self.Lever Pulled`)))
    (goto _label))
  (:`Released`
    (`/Engine/EditorBlueprintResources/StandardMacros.IsValid` _other_actors_are_controlled_by_this_actor :!label _label_2
      (:`Is Valid`
        (if (`KismetSystemLibrary.DoesImplementInterface` _other_actors_are_controlled_by_this_actor "/Game/Blueprints/TogglebleObject.TogglebleObject_C")
          (`self.DisableInput` (`GameplayStatics.GetPlayerController` 0))
          (message `/Game/Blueprints/TogglebleObject.Turn Off` _other_actors_are_controlled_by_this_actor null))))))

(event `self.Box.OnComponentEndOverlap`
  (params (OverlappedComponent :type "PrimitiveComponent Object Reference") (OtherActor :type "Actor Object Reference") (OtherComp :type "PrimitiveComponent Object Reference") (OtherBodyIndex :type Integer))
  (goto _label_2))

(fn `UserConstructionScript`)