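; Elevator actor that builds its own shaft and carries a Mover component up to a height set by floor count.
; The construction script adds instanced walls per floor, leaving openings at the front on the bottom floor and the back on the top.
; The Elevate timeline drives Mover height, with play rate scaled for constant velocity.
; TurnOn or Interact inside the box raises it; TurnOff or the player leaving reverses it.
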(event `/Game/Blueprints/TogglebleObject.Turn On`
  (params (PlayerInteract1 :type "/Game/Blueprints/FirstPersonCharacter Object Reference"))
  (bind (_direction _percent) (`Timeline|Elevate` :!label _label)
    (:`Update`
      (`SceneComponent.K2_SetRelativeLocation` (`self.Mover`) (`KismetMathLibrary.MakeVector` 0.0 0.0 (* _percent (`self.Max Height`))) false false))))

(event `InputAction|Interact`
  (params (Key :type "Key Structure"))
  (:`Pressed`
    (goto _label)))

(event `/Game/Blueprints/TogglebleObject.Turn Off`
  (params (PlayerInteract2 :type "/Game/Blueprints/FirstPersonCharacter Object Reference"))
  (goto _label :!via `Reverse`))

(event `self.Box.OnComponentBeginOverlap`
  (params (OverlappedComponent :type "PrimitiveComponent Object Reference") (OtherActor :type "Actor Object Reference") (OtherComp :type "PrimitiveComponent Object Reference") (OtherBodyIndex :type Integer) (bFromSweep :type Boolean) (SweepResult :type "HitResult Structure (by ref)"))
  ;[1 1 1] Enable / Disable
  (cast `/Game/Blueprints/FirstPersonCharacter` OtherActor)
  (`self.EnableInput` (`GameplayStatics.GetPlayerController` 0)))

(event `self.ReceiveBeginPlay`
  (`TimelineComponent.SetPlayRate` (`self.Elevate`) (/ (`self.Velocity`) (`self.Max Height`))))

(event `self.Box.OnComponentEndOverlap`
  (params (OverlappedComponent :type "PrimitiveComponent Object Reference") (OtherActor :type "Actor Object Reference") (OtherComp :type "PrimitiveComponent Object Reference") (OtherBodyIndex :type Integer))
  ;[1 1 1] Enable / Disable
  (cast `/Game/Blueprints/FirstPersonCharacter` OtherActor)
  (`self.DisableInput` (`GameplayStatics.GetPlayerController` 0))
  (goto _label :!via `Reverse`))

(fn `UserConstructionScript`
  (locals (`Current Floor` :type Integer) (`current z` :type "Float (double-precision)"))
  (set `self.Max Height` (* (`self.Max Floors`) 400.0))
  (for _index (range (+ (`self.Max Floors`) 1))
    (bind _output_get (set `local.Current Floor` _index))
    (set `local.current z` (* _output_get 400.0))
    (`InstancedStaticMeshComponent.AddInstance` (`self.Wall Instance Mesh`) (`KismetMathLibrary.MakeTransform` (`KismetMathLibrary.MakeVector` 0.0 200.0 (`local.current z`))))
    (`InstancedStaticMeshComponent.AddInstance` (`self.Wall Instance Mesh`) (`KismetMathLibrary.MakeTransform` (`KismetMathLibrary.MakeVector` 0.0 -200.0 (`local.current z`))))
    (if (not (== (`local.Current Floor`) (`self.Max Floors`)))
      (`InstancedStaticMeshComponent.AddInstance` (`self.Wall Instance Mesh`) (`KismetMathLibrary.MakeTransform` (`KismetMathLibrary.MakeVector` 0.0 -195.0 (`local.current z`)) (struct :`Yaw` 90.0))) ; Back Wall
    )
    (if (!= (`local.Current Floor`) 0)
      (`InstancedStaticMeshComponent.AddInstance` (`self.Wall Instance Mesh`) (`KismetMathLibrary.MakeTransform` (`KismetMathLibrary.MakeVector` 400.0 -200.0 (`local.current z`)) (struct :`Yaw` 90.0))) ; Front Wall
    )))