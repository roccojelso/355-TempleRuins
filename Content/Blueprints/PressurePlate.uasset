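; Pressure plate actor that switches another actor on while the first-person character stands on it.
; Box overlap begin and end events swap the Plate mesh between active and inactive materials.
; They send TurnOn or TurnOff messages to a single referenced actor through the TogglebleObject interface.
; Nothing happens, not even the material change, unless that reference is valid and implements the interface.
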(event `self.Box.OnComponentBeginOverlap`
  (params (OverlappedComponent :type "PrimitiveComponent Object Reference") (OtherActor :type "Actor Object Reference") (OtherComp :type "PrimitiveComponent Object Reference") (OtherBodyIndex :type Integer) (bFromSweep :type Boolean) (SweepResult :type "HitResult Structure (by ref)"))
  (bind _other_actors_controlled_by_this_actor (`self.Other Actors controlled by this Actor`))
  (`/Engine/EditorBlueprintResources/StandardMacros.IsValid` _other_actors_controlled_by_this_actor
    (:`Is Valid`
      (if (`KismetSystemLibrary.DoesImplementInterface` _other_actors_controlled_by_this_actor "/Game/Blueprints/TogglebleObject.TogglebleObject_C")
        (cast `/Game/Blueprints/FirstPersonCharacter` OtherActor)
        (`PrimitiveComponent.SetMaterial` (`self.Plate`) 0 (`self.ActiveMaterial`))
        (message `/Game/Blueprints/TogglebleObject.Turn On` _other_actors_controlled_by_this_actor null)))))

(event `self.Box.OnComponentEndOverlap`
  (params (OverlappedComponent :type "PrimitiveComponent Object Reference") (OtherActor :type "Actor Object Reference") (OtherComp :type "PrimitiveComponent Object Reference") (OtherBodyIndex :type Integer))
  (bind _other_actors_controlled_by_this_actor (`self.Other Actors controlled by this Actor`))
  (`/Engine/EditorBlueprintResources/StandardMacros.IsValid` _other_actors_controlled_by_this_actor
    (:`Is Valid`
      (if (`KismetSystemLibrary.DoesImplementInterface` _other_actors_controlled_by_this_actor "/Game/Blueprints/TogglebleObject.TogglebleObject_C")
        (cast `/Game/Blueprints/FirstPersonCharacter` OtherActor)
        (`PrimitiveComponent.SetMaterial` (`self.Plate`) 0 (`self.InActiveMaterial`))
        (message `/Game/Blueprints/TogglebleObject.Turn Off` _other_actors_controlled_by_this_actor null)))))

(fn `UserConstructionScript`)