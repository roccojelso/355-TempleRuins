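; Interactive door Blueprint that the player opens and closes with the E key while standing near it.
; Overlapping the Box enables input for the first player controller, and leaving it disables input.
; E toggles a DoorClosed flag and plays or reverses the OpenAndClose timeline, whose track sets the Door's absolute world yaw.
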(event `self.Box.OnComponentBeginOverlap`
  (params (OverlappedComponent :type "PrimitiveComponent Object Reference") (OtherActor :type "Actor Object Reference") (OtherComp :type "PrimitiveComponent Object Reference") (OtherBodyIndex :type Integer) (bFromSweep :type Boolean) (SweepResult :type "HitResult Structure (by ref)"))
  ;[1 1 1] Enable/Disable
  (`self.EnableInput` (`GameplayStatics.GetPlayerController` 0)))

(event `Key|E`
  (params (Key :type "Key Structure"))
  ;[1 1 1] E Input - Activate Open and Close Animation
  (:`Pressed`
    (if (`self.Door Closed`)
      (set `self.Door Closed` false)
      (bind (_direction _open_close) (`Timeline|Open and Close` :!label _label)
        (:`Update`
          (`SceneComponent.K2_SetWorldRotation` (`self.Door`) (`KismetMathLibrary.MakeRotator` 0.0 0.0 _open_close) false false)))
      (else
        (set `self.Door Closed` true)
        (goto _label :!via `Reverse`)))))

(event `self.Box.OnComponentEndOverlap`
  (params (OverlappedComponent :type "PrimitiveComponent Object Reference") (OtherActor :type "Actor Object Reference") (OtherComp :type "PrimitiveComponent Object Reference") (OtherBodyIndex :type Integer))
  ;[1 1 1] Enable/Disable
  (`self.DisableInput` (`GameplayStatics.GetPlayerController` 0)))

(fn `UserConstructionScript`)